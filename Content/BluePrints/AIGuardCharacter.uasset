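; AI guard character that patrols a looping list of waypoints on the navmesh.
; BeginPlay caches its AI controller and sets the first target to its own navmesh-projected location.
; Tick reissues MoveToLocation; on failure or arrival it waits three seconds, then advances the index and projects that waypoint onto the navmesh.
; An index past the array length resets to zero without updating the target that pass.
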(event `self.ReceiveBeginPlay`
  ;[1 1 1] At the begging of the level its starts finding target location
  (set `self.AI Contoller` (`AIBlueprintHelperLibrary.GetAIController` self))
  (set `self.TargetLocation` (`NavigationSystemV1.K2_ProjectPointToNavigation` (`self.K2_GetActorLocation`) (`self.NavData`))))

(event `self.ReceiveTick`
  (params (DeltaSeconds :type "Float (single-precision)"))
  ;[1 1 1] On every tick the AI will goto location path  and if it fails or goal is complete it will  contunie to go through each waypoint on loop and gets actor location based on nav data and point to navigation
  (bind _returnvalue (`AIController.MoveToLocation` (`self.AI Contoller`) (`self.TargetLocation`) -1.0 true true false true null true))
  (switch `EPathFollowingRequestResult` _returnvalue
    (:`Failed`
      _)
    (:`AlreadyAtGoal`
      _))
  (`KismetSystemLibrary.Delay` 3.0)
  (`/Engine/EditorBlueprintResources/StandardMacros.IncrementInt` (`self.CurrentWaypoint`)
    (:`  `
      (if (<= (`self.CurrentWaypoint`) (`KismetArrayLibrary.Array_Length` (`self.Waypoints`)))
        (set `self.TargetLocation` (`NavigationSystemV1.K2_ProjectPointToNavigation` (`self.K2_GetActorLocation` (`|GetArrayItem` (`self.Waypoints`) (`self.CurrentWaypoint`))) (`self.NavData`)))
        (else
          (set `self.CurrentWaypoint` 0))))))

(fn `UserConstructionScript`)