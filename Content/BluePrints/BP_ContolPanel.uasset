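; BP_ContolPanel is an interactable control panel that unlocks a linked door when the player presses E nearby.
; Beginning and ending overlap swap a referenced TextRender actor between tutorial and exit text and toggle input for player controller 0, without checking which actor overlapped.
; Releasing E clears the door's Islocked flag and shows unlocked text as feedback.
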(event `self.ReceiveBeginPlay`
  ;[1 1 1] OnBeginPlay,Set Text To EmpyText
  (`TextRenderComponent.K2_SetText` (`TextRenderActor.TextRender` (`self.TextRenderActorToChange`)) (`KismetTextLibrary.Conv_StringToText` (`self.ExitText`))))

(event `self.ReceiveActorBeginOverlap`
  (params (OtherActor :type "Actor Object Reference"))
  ;[1 1 1] On Actor Begin Overlap,Change Text to Tutorial Text and lsiten for keyboard input
  (`TextRenderComponent.K2_SetText` (`TextRenderActor.TextRender` (`self.TextRenderActorToChange`)) (`KismetTextLibrary.Conv_StringToText` (`self.TutorialText`)))
  (`self.EnableInput` self (`GameplayStatics.GetPlayerController` 0)))

(event `self.ReceiveActorEndOverlap`
  (params (OtherActor :type "Actor Object Reference"))
  ;[1 1 1] On ActorEndOverlap,Change text to exit text and stop listening for keyboard input
  (`TextRenderComponent.K2_SetText` (`TextRenderActor.TextRender` (`self.TextRenderActorToChange`)) (`KismetTextLibrary.Conv_StringToText` (`self.ExitText`)))
  (`self.DisableInput` self (`GameplayStatics.GetPlayerController` 0)))

(event `Key|E`
  (params (Key :type "Key Structure"))
  ;[1 1 1] On E, Unlock the Door and provide feedback
  (:`Released`
    (set `/Game/BluePrints/BP_LockableDoor.islocked` false (`self.Door to Unlock`))
    (`TextRenderComponent.K2_SetText` (`TextRenderActor.TextRender` (`self.TextRenderActorToChange`)) (`KismetTextLibrary.Conv_StringToText` (`self.Unlocked Text`)))))

(fn `UserConstructionScript`)