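; BP_Doexample is an elevator actor that demonstrates a DoN node, rising only the first three times the player pawn enters its trigger box.
; A timeline lerps the mesh's relative Z from the height cached on BeginPlay to that height multiplied by ElevatorEnd.
; End overlap reverses the timeline for any actor, without a player check.
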(event `self.ReceiveBeginPlay`
  (bind (_relativelocation_x _relativelocation_y _relativelocation_z) (`KismetMathLibrary.BreakVector` (`SceneComponent.RelativeLocation` (`self.StaticMeshComponent1`))))
  ;[1 1 1] At the begging of play the elevayor will start at the elevator start
  (set `self.ElevatorStart` _relativelocation_z))

(event `self.Box.OnComponentBeginOverlap`
  (params (OverlappedComponent :type "PrimitiveComponent Object Reference") (OtherActor :type "Actor Object Reference") (OtherComp :type "PrimitiveComponent Object Reference") (OtherBodyIndex :type Integer) (bFromSweep :type Boolean) (SweepResult :type "HitResult Structure (by ref)"))
  (bind _elevatorstart (`self.ElevatorStart`))
  ;[1 1 1] At the begin of the overlap it will get player pawn and branch and do n when enter
  (if (== OtherActor (`GameplayStatics.GetPlayerPawn` 0))
    (`/Engine/EditorBlueprintResources/StandardMacros.Do N` 3
      (:`Exit`
        ;[1 1 1] Onupdate it will move the elevator and set the realtive location and new location based on teh lerp.
        (bind (_direction _elevatorheight) (`Timeline|MoveElevator` :!via `PlayFromStart` :!label _label)
          (:`Update`
            (`SceneComponent.K2_SetRelativeLocation` (`self.StaticMeshComponent1`) (`KismetMathLibrary.MakeVector` 0.0 0.0 (`KismetMathLibrary.Lerp` _elevatorstart (* _elevatorstart (`self.ElevatorEnd`)) _elevatorheight)) false false)))))))

(event `self.Box.OnComponentEndOverlap`
  (params (OverlappedComponent :type "PrimitiveComponent Object Reference") (OtherActor :type "Actor Object Reference") (OtherComp :type "PrimitiveComponent Object Reference") (OtherBodyIndex :type Integer))
  ;[1 1 1] When player leaves the elevator will go in reverse
  (goto _label :!via `Reverse`))

(fn `UserConstructionScript`)