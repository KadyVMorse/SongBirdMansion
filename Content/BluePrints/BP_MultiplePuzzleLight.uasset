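; BP_MultiplePuzzleLight is a point light that indicates whether every puzzle in its Targets array is solved.
; Each Tick it loops over the targets, stopping at the first one whose Succuess flag is false.
; It then sets the light green when all targets succeed, or dark red otherwise.
; An empty Targets array also shows green.
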(event `self.ReceiveTick`
  (params (DeltaSeconds :type "Float (single-precision)"))
  (bind _pointlightcomponent (`self.PointLightComponent`))
  (set `self.Succues` true)
  (for _array_element (`self.Targets`)
    (if (not (`/Game/BluePrints/BP_TargetLocation.Succuess` _array_element))
      (set `self.Succues` false)
      (break)))
  (if (`self.Succues`)
    (`LightComponent.SetLightColor` _pointlightcomponent (struct :`R` 0.152503 :`G` 1.0 :`A` 1.0) true)
    (else
      (`LightComponent.SetLightColor` _pointlightcomponent (struct :`R` 0.3375 :`G` 0.052234 :`B` 0.044176 :`A` 1.0) true))))

(fn `UserConstructionScript`)