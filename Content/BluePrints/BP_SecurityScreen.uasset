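; BP_SecurityScreen is a security monitor that shows one of three camera views on its static mesh.
; Every Tick, it switches on CameraNumberToShow and applies the matching entry from the Materials array to the mesh's first material slot.
; An out-of-range number resets to the first camera, and nothing in this Blueprint otherwise changes the selection.
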(event `self.ReceiveTick`
  (params (DeltaSeconds :type "Float (single-precision)"))
  ;[1 1 1] When event is ticked it will switch between the cameras
  (switch `int` (`self.CameraNumberToShow`)
    (:`Default`
      ;[1 1 1] Sets the camera to show defult
      (set `self.CameraNumberToShow` 0))
    (:`0`
      ;[1 1 1] Set to Material 0
      (`PrimitiveComponent.SetMaterial` (`self.StaticMeshComponent`) 0 (`|GetArrayItem` (`self.Materials`))))
    (:`1`
      ;[1 1 1] Set to Material 1
      (`PrimitiveComponent.SetMaterial` (`self.StaticMeshComponent`) 0 (`|GetArrayItem` (`self.Materials`) 1)))
    (:`2`
      ;[1 1 1] Set to material 2
      (`PrimitiveComponent.SetMaterial` (`self.StaticMeshComponent`) 0 (`|GetArrayItem` (`self.Materials`) 2)))))

(fn `UserConstructionScript`)