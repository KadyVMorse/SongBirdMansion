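; AI character Blueprint that wanders the navmesh, reacts to sight and sound, and is destroyed when damage depletes its Health.
; Tick continually moves it toward TargetLocation, choosing a random reachable point within WanderRaduis after a three-second delay upon arrival or failure.
; PawnSensing redirects that target to the navmesh-projected position of seen pawns at running speed, or of sufficiently loud noise instigators at walking speed.
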(event `self.ReceiveAnyDamage`
  (params (Damage :type "Float (single-precision)") (DamageType :type "DamageType Object Reference") (InstigatedBy :type "Controller Object Reference") (DamageCauser :type "Actor Object Reference"))
  ;[1 1 1] Everytime we take damge it will minus our current health and if our health is <= to 0 then the actor will be destroyed
  (bind _output_get (set `self.Health` (- (`self.Health`) Damage)))
  (if (<= _output_get 0.0)
    (`self.K2_DestroyActor`)))

(event `self.ReceiveBeginPlay`
  ;[1 1 1] On the begging of the level the AI gets its Target location
  (set `self.AI Contoller` (`AIBlueprintHelperLibrary.GetAIController` self))
  (set `self.TargetLocation` (`self.K2_GetActorLocation`)))

(event `self.ReceiveTick`
  (params (DeltaSeconds :type "Float (single-precision)"))
  ;[1 1 1] On every Frame The AI will follow a path when it meets its goal or fails and it will delay for 3 seconds and when completed will go to next location based on location nav data and wander raduis
  (bind _returnvalue (`AIController.MoveToLocation` (`self.AI Contoller`) (`self.TargetLocation`) -1.0 true true false true null true))
  (switch `EPathFollowingRequestResult` _returnvalue
    (:`Failed`
      _)
    (:`AlreadyAtGoal`
      _))
  (`KismetSystemLibrary.Delay` 3.0)
  (set `self.TargetLocation` (`NavigationSystemV1.K2_GetRandomReachablePointInRadius` (`self.TargetLocation`) (`self.WanderRaduis`) (`self.NavData`) null)))

(event `self.PawnSensing.OnSeePawn`
  (params (Pawn :type "Pawn Object Reference"))
  ;[1 1 1] When the AI Sees the player it will run towards player location and then follow them if fully spotted
  (set `CharacterMovementComponent.MaxWalkSpeed` 600.0 (`self.CharacterMovement`))
  (set `self.TargetLocation` (`NavigationSystemV1.K2_ProjectPointToNavigation` (`self.K2_GetActorLocation` Pawn) (`self.NavData`))))

(event `self.PawnSensing.OnHearNoise`
  (params (Instigator :type "Pawn Object Reference") (Location :type "Vector Structure (by ref)") (Volume :type "Float (single-precision)"))
  ;[1 1 1] When AI hears noise it will investigate and walk towards the area that they heard noise based on Actors location and nav data
  (if (>= Volume (`self.HearingCutOff`))
    (set `CharacterMovementComponent.MaxWalkSpeed` 100.0 (`self.CharacterMovement`))
    (set `self.TargetLocation` (`NavigationSystemV1.K2_ProjectPointToNavigation` (`self.K2_GetActorLocation` Instigator) (`self.NavData`)))))

(fn `UserConstructionScript`)