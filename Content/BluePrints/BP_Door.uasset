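; BP_Door is a door actor that swings open when something overlaps its trigger box and closes when the overlap ends.
; At BeginPlay the door is set to its closed yaw.
; Box overlap events play and reverse the DoorOpen timeline, whose RotationPercent track lerps the door's relative yaw between ClosedRotation and OpenRotation.
; The overlap events do not filter for the player.
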(event `self.ReceiveBeginPlay`
  ;[1 1 1] Sets the door to certain postion at start of level
  (`SceneComponent.K2_SetRelativeRotation` (`self.Door`) (`KismetMathLibrary.MakeRotator` 0.0 0.0 (`self.ClosedRotation`)) false false))

(event `self.Box.OnComponentBeginOverlap`
  (params (OverlappedComponent :type "PrimitiveComponent Object Reference") (OtherActor :type "Actor Object Reference") (OtherComp :type "PrimitiveComponent Object Reference") (OtherBodyIndex :type Integer) (bFromSweep :type Boolean) (SweepResult :type "HitResult Structure (by ref)"))
  ;[1 1 1] The timemode plays when the player enters the collsion box
  ;[1 1 1] On update it sets the realtive rotation of the door and sets the rotation percent and lerps the closed and open rotation
  (bind (_direction _rotationpercent) (`Timeline|DoorOpen` :!label _label)
    (:`Update`
      (`SceneComponent.K2_SetRelativeRotation` (`self.Door`) (`KismetMathLibrary.MakeRotator` 0.0 0.0 (`KismetMathLibrary.Lerp` (`self.ClosedRotation`) (`self.OpenRotation`) _rotationpercent)) false false))))

(event `self.Box.OnComponentEndOverlap`
  (params (OverlappedComponent :type "PrimitiveComponent Object Reference") (OtherActor :type "Actor Object Reference") (OtherComp :type "PrimitiveComponent Object Reference") (OtherBodyIndex :type Integer))
  ;[1 1 1] The timemode is played in reverse when the player leaves the box
  (goto _label :!via `Reverse`))

(fn `UserConstructionScript`)