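; BP_CharacterSwapTrigger is a trigger actor that lets the player switch control to another pawn by pressing E.
; It disables its own input at BeginPlay and on end overlap, and enables it for player controller 0 when any actor begins overlapping.
; Pressing E makes that controller unpossess its pawn, possess PawnToPossess, then disables the trigger's input again.
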(event `self.ReceiveBeginPlay`
  ;[1 1 1] At the begging of play and at the end of overlap it disables input
  (`self.DisableInput` (`GameplayStatics.GetPlayerController` 0) :!label _label))

(event `self.ReceiveActorEndOverlap`
  (params (OtherActor :type "Actor Object Reference"))
  ;[1 1 1] At the begging of play and at the end of overlap it disables input
  (goto _label))

(event `self.ReceiveActorBeginOverlap`
  (params (OtherActor :type "Actor Object Reference"))
  ;[1 1 1] On overlap the player can have input
  (`self.EnableInput` (`GameplayStatics.GetPlayerController` 0)))

(event `Key|E`
  (params (Key :type "Key Structure"))
  (bind _returnvalue (`GameplayStatics.GetPlayerController` 0))
  ;[1 1 1] When press E the player can posses and unposses when in collision box but input will be taken away when the player switch.
  (:`Pressed`
    (`Controller.UnPossess` _returnvalue)
    (`Controller.Possess` _returnvalue (`self.PawnToPossess`))
    (`self.DisableInput` _returnvalue)))

(fn `UserConstructionScript`)