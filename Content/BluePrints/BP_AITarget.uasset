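; BP_AITarget is a trigger actor that lets the player send all AI characters to their current location.
; It enables its input while the player pawn overlaps it and disables it at BeginPlay and when the overlap ends.
; Pressing E projects the player pawn's location onto the navigation data and writes the result to TargetLocation on every AICharacter in the level.
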(event `self.ReceiveBeginPlay`
  ;[1 1 1] At the begginig of level and when the AI ovelaps then the input is disabled
  (`self.DisableInput` (`GameplayStatics.GetPlayerController` 0) :!label _label))

(event `self.ReceiveActorEndOverlap`
  (params (OtherActor :type "Actor Object Reference"))
  ;[1 1 1] At the begginig of level and when the AI ovelaps then the input is disabled
  (if (== OtherActor (`GameplayStatics.GetPlayerPawn` 0))
    (goto _label)))

(event `Key|E`
  (params (Key :type "Key Structure"))
  ;[1 1 1] When key E is pressed every AI will go to Target location
  (:`Pressed`
    (bind _outactors (`GameplayStatics.GetAllActorsOfClass` "/Game/BluePrints/AICharacter.AICharacter_C"))
    (for _array_element _outactors
      (set `/Game/BluePrints/AICharacter.TargetLocation` (`NavigationSystemV1.K2_ProjectPointToNavigation` (`self.K2_GetActorLocation` (`GameplayStatics.GetPlayerPawn` 0)) (`self.NavData`)) _array_element))))

(event `self.ReceiveActorBeginOverlap`
  (params (OtherActor :type "Actor Object Reference"))
  ;[1 1 1] If the player overlaps with the trigger than it enables input
  (if (== OtherActor (`GameplayStatics.GetPlayerPawn` 0))
    (`self.EnableInput` (`GameplayStatics.GetPlayerController` 0))))

(fn `UserConstructionScript`)