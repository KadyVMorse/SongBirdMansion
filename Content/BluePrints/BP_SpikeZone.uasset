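; BP_SpikeZone is a hazard actor that deals continuous damage to Characters standing inside its Box trigger.
; Box begin and end overlap events add and remove Characters in a unique CharacterInSpikes array.
; Each Tick applies damage to every listed Character, scaling DPS by DeltaSeconds so the rate stays frame-rate independent.
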(event `self.ReceiveTick`
  (params (DeltaSeconds :type "Float (single-precision)"))
  ;[1 1 1] For every second the spikes are on loop to cause damage  to the list of characters
  (for _array_element (`self.CharacterInSpikes`)
    (`GameplayStatics.ApplyDamage` _array_element (* (`self.DPS`) DeltaSeconds) null self)))

(event `self.Box.OnComponentBeginOverlap`
  (params (OverlappedComponent :type "PrimitiveComponent Object Reference") (OtherActor :type "Actor Object Reference") (OtherComp :type "PrimitiveComponent Object Reference") (OtherBodyIndex :type Integer) (bFromSweep :type Boolean) (SweepResult :type "HitResult Structure (by ref)"))
  ;[1 1 1] When Character overlap we are going to add it to an unique list
  (bind _ascharacter (cast `Character` OtherActor))
  (`KismetArrayLibrary.Array_AddUnique` (`self.CharacterInSpikes`) _ascharacter))

(event `self.Box.OnComponentEndOverlap`
  (params (OverlappedComponent :type "PrimitiveComponent Object Reference") (OtherActor :type "Actor Object Reference") (OtherComp :type "PrimitiveComponent Object Reference") (OtherBodyIndex :type Integer))
  ;[1 1 1] When Character stops overlap we are going to remove it
  (bind _ascharacter (cast `Character` OtherActor))
  (`KismetArrayLibrary.Array_RemoveItem` (`self.CharacterInSpikes`) _ascharacter))

(fn `UserConstructionScript`)