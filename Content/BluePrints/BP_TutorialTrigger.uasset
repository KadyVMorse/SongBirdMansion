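; Trigger actor that shows tutorial text in the level through a referenced TextRender actor.
; Beginning an overlap sets that actor's text to TutorialText, and ending one sets it to ExitText.
; Neither overlap event filters the other actor or checks that the reference is valid.
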(event `self.ReceiveActorBeginOverlap`
  (params (OtherActor :type "Actor Object Reference"))
  (`TextRenderComponent.K2_SetText` (`TextRenderActor.TextRender` (`self.TextRenderActorToChange`)) (`KismetTextLibrary.Conv_StringToText` (`self.TutorialText`))))

(event `self.ReceiveActorEndOverlap`
  (params (OtherActor :type "Actor Object Reference"))
  (`TextRenderComponent.K2_SetText` (`TextRenderActor.TextRender` (`self.TextRenderActorToChange`)) (`KismetTextLibrary.Conv_StringToText` (`self.ExitText`))))

(fn `UserConstructionScript`)