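; A trigger box Blueprint that switches a referenced particle effect on while an actor overlaps it.
; The effect's particle system is deactivated at BeginPlay, activated on begin overlap without a reset, and deactivated again on end overlap, with no filtering of the overlapping actor.
; An unconnected branch on Spooky, which either prints a message or plays BookMantinee, is left in the graph and never runs.
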(event `self.ReceiveBeginPlay`
  (`ActorComponent.Deactivate` (`Emitter.ParticleSystemComponent` (`self.Particule effect`)) :!label _label))

(event `self.ReceiveActorEndOverlap`
  (params (OtherActor :type "Actor Object Reference"))
  (goto _label))

(event `self.ReceiveActorBeginOverlap`
  (params (OtherActor :type "Actor Object Reference"))
  (`ActorComponent.Activate` (`Emitter.ParticleSystemComponent` (`self.Particule effect`)) false))

(fn `UserConstructionScript`)